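; Square painting actor that displays an image downloaded from a URL and can be opened full screen.
; On BeginPlay, if a URL is set, it downloads the image and applies it to the ImageTexture of the Painting component's Painting_WB_Sqiare widget.
; Interact creates a FullScreen_Square widget and adds it to the viewport, without passing it the downloaded image.
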(event `self.ReceiveBeginPlay`
  (if (not (`KismetStringLibrary.IsEmpty` (`self.URL`)))
    (bind _texture (`AsyncTaskDownloadImage.DownloadImage` (`self.URL`))
      (:`OnSuccess`
        (bind _aspainting_wb_sqiare (cast `/Game/Blueprints/Painting_WB_Sqiare` (`WidgetComponent.GetWidget` (`self.Painting`))))
        (`Image.SetBrushFromTextureDynamic` (`/Game/Blueprints/Painting_WB_Sqiare.Image_Texture` _aspainting_wb_sqiare) _texture false)))))

(event `/Game/Blueprints/Interfaces/Interact.Interact`
  (params (Base_BP :type "/Game/Blueprints/Base_BP Object Reference"))
  (bind _returnvalue (`|CreateWidget` "/Game/Blueprints/FullScreen_Square.FullScreen_Square_C"))
  (`UserWidget.AddToViewport` _returnvalue 0))

(fn `UserConstructionScript`)