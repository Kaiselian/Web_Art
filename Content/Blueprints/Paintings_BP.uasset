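; Interactable painting actor that shows a web image on an in-world widget and can open a full-screen widget.
; On BeginPlay, a non-empty URL is downloaded and the resulting texture is set as the image brush on the Painting component's Painting_WB widget.
; Interact creates a FullScreen widget and adds it to the viewport, without passing it the downloaded texture.
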(event `self.ReceiveBeginPlay`
  (if (not (`KismetStringLibrary.IsEmpty` (`self.URL`)))
    (bind _texture (`AsyncTaskDownloadImage.DownloadImage` (`self.URL`))
      (:`OnSuccess`
        (bind _aspainting_wb (cast `/Game/Blueprints/Painting_WB` (`WidgetComponent.GetWidget` (`self.Painting`))))
        (`Image.SetBrushFromTextureDynamic` (`/Game/Blueprints/Painting_WB.Image_Texture` _aspainting_wb) _texture false)))))

(event `/Game/Blueprints/Interfaces/Interact.Interact`
  (params (Base_BP :type "/Game/Blueprints/Base_BP Object Reference"))
  (bind _returnvalue (`|CreateWidget` "/Game/Blueprints/FullScreen.FullScreen_C"))
  (`UserWidget.AddToViewport` _returnvalue 0))

(fn `UserConstructionScript`)